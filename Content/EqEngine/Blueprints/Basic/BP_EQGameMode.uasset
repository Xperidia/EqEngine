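; BP_EQGameMode is the game mode that holds back match start until loading finishes and triggers player loading on restart.
; ReadyToStartMatch returns the IsLoadingFinished flag from BP_EQGameStateBase, or false if the game state is not that class.
; OnRestartPlayer casts the player to BP_EQPlayerController and calls ClientLoadPlayer on it.
; UI_GetSocialState and GetSocialComponent are stubs returning empty defaults.
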(event `Event OnRestartPlayer`
  (params (NewPlayer :type "Controller Object Reference"))
  ;[0.845 0.1098 0.1098] Server: Load Connected Players When Ready
  (bind _asbp_eqplayer_controller (cast `/Game/EqEngine/Blueprints/Basic/BP_EQPlayerController` NewPlayer))
  (`/Game/EqEngine/Blueprints/Basic/BP_EQPlayerController.Client_LoadPlayer` _asbp_eqplayer_controller))

(fn `GetSocialComponent`
  (returns (SocialSystemReference :type "/Game/AdvancedSocialSystem/Blueprints/Social/SocialSystemComponent Object Reference"))
  (return null))

(fn `ReadyToStartMatch`
  (returns (ReturnValue :type Boolean))
  (bind _asbp_eqgame_state_base (cast `/Game/EqEngine/Blueprints/Basic/BP_EQGameStateBase` (`GameplayStatics.GetGameState`))
    (:`then`
      (return (`/Game/EqEngine/Blueprints/Basic/BP_EQGameStateBase.IsLoadingFinished` _asbp_eqgame_state_base)))
    (:`CastFailed`
      (return false))))

(fn `UI_GetSocialState`
  (returns (SocialID :type Integer) (SocialName :type String) (PartyID :type Integer) (GuildID :type Integer) (GuildName :type String) (GeneralID :type Integer) (TradeID :type Integer))
  (return 0 "" 0 0 "" 0 0))

(fn `UserConstructionScript`)