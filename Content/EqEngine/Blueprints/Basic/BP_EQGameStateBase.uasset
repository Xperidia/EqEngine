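; Game state base that holds the Players, Guilds and Parties registries for EqEngine.
; On authority, BeginPlay fills guilds and players from demo data tables, then sets IsLoadingFinished after a placeholder delay to allow player spawning.
; Array index doubles as record ID: loads write at the stored ID, while create/add functions append and write the new index back.
; These writes are authority-gated, except UpdatePlayerStatus, which replaces a player's PlayerState without that check.
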(event `self.ReceiveBeginPlay`
  (`/Engine/EditorBlueprintResources/ActorMacros.Switch Has Authority`
    (:`Authority`
      (`|ExecutionSequence`
        (:`then_0`
          ;[0.845 0.1098 0.1098] Load Demo [Guilds]
          (bind _outrownames (`DataTableFunctionLibrary.GetDataTableRowNames` "/Game/AdvancedSocialSystem/Blueprints/Social/ListGuilds.ListGuilds"))
          (`KismetArrayLibrary.Array_Resize` (`self.Guilds`) (`KismetArrayLibrary.Array_Length` _outrownames))
          (for _array_element _outrownames
            (bind _returnvalue (`|GetDataTableRow` "/Game/AdvancedSocialSystem/Blueprints/Social/ListGuilds.ListGuilds" _array_element)
              (:`then`
                (`self.Server_LoadGuild` _returnvalue)))))
        (:`then_1`
          ;[0.845 0.1098 0.1098] Load Demo [Player List]
          (bind _outrownames_2 (`DataTableFunctionLibrary.GetDataTableRowNames` "/Game/AdvancedSocialSystem/Blueprints/Social/ListPlayers.ListPlayers"))
          (`KismetArrayLibrary.Array_Resize` (`self.Players`) (`KismetArrayLibrary.Array_Length` _outrownames_2))
          (for _array_element_2 _outrownames_2
            (bind _returnvalue_2 (`|GetDataTableRow` "/Game/AdvancedSocialSystem/Blueprints/Social/ListPlayers.ListPlayers" _array_element_2)
              (:`then`
                (`self.Server_LoadPlayer` _returnvalue_2)))))
        (:`then_2`
          ;[0.845 0.1098 0.1098] Allow Players To Spawn In
          (`KismetSystemLibrary.Delay` 0.0) ; Simulate Server Loading
          (set `self.IsLoadingFinished` true))))))

(fn `Server_AddPlayer`
  (params (PlayerInfo :type "/Game/AdvancedSocialSystem/Blueprints/Social/SPlayer Structure"))
  (returns (PlayerID :type Integer))
  (locals (LocalID :type Integer))
  (bind (_id _name _guildid _partyid _playerstate) (break `/Game/AdvancedSocialSystem/Blueprints/Social/SPlayer` PlayerInfo))
  (bind _localid (`local.LocalID`))
  (`/Engine/EditorBlueprintResources/ActorMacros.Switch Has Authority`
    (:`Authority`
      (bind _returnvalue (`KismetArrayLibrary.Array_Add` (`self.Players`) PlayerInfo))
      (set `local.LocalID` _returnvalue)
      (`KismetArrayLibrary.Array_Set` (`self.Players`) _localid (make `/Game/AdvancedSocialSystem/Blueprints/Social/SPlayer` _localid _name _guildid _partyid _playerstate))
      (return (`local.LocalID`)))
    (:`Remote`
      (return -1))))

(fn `Server_CreateGuild`
  (params (GuildInfo :type "/Game/AdvancedSocialSystem/Blueprints/Social/SGuild Structure"))
  (returns (GuildID :type Integer))
  (locals (LocalID :type Integer))
  (bind (_id _name _motd _leader _members) (break `/Game/AdvancedSocialSystem/Blueprints/Social/SGuild` GuildInfo))
  (bind _localid (`local.LocalID`))
  (`/Engine/EditorBlueprintResources/ActorMacros.Switch Has Authority`
    (:`Authority`
      (bind _returnvalue (`KismetArrayLibrary.Array_Add` (`self.Guilds`) GuildInfo))
      (set `local.LocalID` _returnvalue)
      (`KismetArrayLibrary.Array_Set` (`self.Guilds`) _localid (make `/Game/AdvancedSocialSystem/Blueprints/Social/SGuild` _localid _name _motd _leader _members))
      (return (`local.LocalID`)))
    (:`Remote`
      (return -1))))

(fn `Server_CreateParty`
  (params (PartyInfo :type "/Game/AdvancedSocialSystem/Blueprints/Social/SParty Structure"))
  (returns (PartyID :type Integer))
  (locals (LocalID :type Integer))
  (bind (_id _leader _members) (break `/Game/AdvancedSocialSystem/Blueprints/Social/SParty` PartyInfo))
  (bind _localid (`local.LocalID`))
  (`/Engine/EditorBlueprintResources/ActorMacros.Switch Has Authority`
    (:`Authority`
      (bind _returnvalue (`KismetArrayLibrary.Array_Add` (`self.Parties`) PartyInfo))
      (set `local.LocalID` _returnvalue)
      (`KismetArrayLibrary.Array_Set` (`self.Parties`) _localid (make `/Game/AdvancedSocialSystem/Blueprints/Social/SParty` _localid _leader _members))
      (return (`local.LocalID`)))
    (:`Remote`
      (return 0))))

(fn `Server_LoadGuild`
  (params (GuildInfo :type "/Game/AdvancedSocialSystem/Blueprints/Social/SGuild Structure"))
  (locals (LocalID :type Integer))
  (bind (_id _name _motd _leader _members) (break `/Game/AdvancedSocialSystem/Blueprints/Social/SGuild` GuildInfo))
  (`/Engine/EditorBlueprintResources/ActorMacros.Switch Has Authority`
    (:`Authority`
      (`KismetArrayLibrary.Array_Set` (`self.Guilds`) _id (make `/Game/AdvancedSocialSystem/Blueprints/Social/SGuild` _id _name _motd _leader _members) true))))

(fn `Server_LoadPlayer`
  (params (PlayerInfo :type "/Game/AdvancedSocialSystem/Blueprints/Social/SPlayer Structure"))
  (locals (LocalID :type Integer))
  (bind (_id _name _guildid _partyid _playerstate) (break `/Game/AdvancedSocialSystem/Blueprints/Social/SPlayer` PlayerInfo))
  (`/Engine/EditorBlueprintResources/ActorMacros.Switch Has Authority`
    (:`Authority`
      (`KismetArrayLibrary.Array_Set` (`self.Players`) _id (make `/Game/AdvancedSocialSystem/Blueprints/Social/SPlayer` _id _name _guildid _partyid _playerstate) true))))

(fn `UpdatePlayerStatus`
  (params (PlayerInfo :type Integer) (PlayerState :type "/Game/EqEngine/Blueprints/Basic/BP_EQPlayerState Object Reference"))
  (locals (LocalPlayerID :type Integer))
  (bind _players (`self.Players`))
  (bind (_id _name _guildid _partyid) (break `/Game/AdvancedSocialSystem/Blueprints/Social/SPlayer` (`KismetArrayLibrary.Array_Get` _players (`local.LocalPlayerID`))))
  (set `local.LocalPlayerID` PlayerInfo)
  (`KismetArrayLibrary.Array_Set` _players (`local.LocalPlayerID`) (make `/Game/AdvancedSocialSystem/Blueprints/Social/SPlayer` _id _name _guildid _partyid PlayerState)))

(fn `UserConstructionScript`)