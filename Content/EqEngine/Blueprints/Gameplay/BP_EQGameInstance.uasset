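; BP_EQGameInstance is the game instance that manages multiplayer sessions, the main menu and the loading screen.
; HostGame stores server settings, creates a session and opens FirstPersonExampleMap as a listen server, while JoinGame joins a search result and DestroySession tears the session down.
; Menu and loading widgets are created lazily and reused.
; Session, client network and travel failures route to Error, though it and both string converters are empty stubs.
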(event `self.HandleNetworkError`
  (params (FailureType :type "ENetworkFailure Enum" :default "NetDriverAlreadyExists") (bIsServer :type Boolean))
  ;[1 1 1] Gère NetworkError & TravelError
  (if (not bIsServer)
    (`self.Error` (`self.NetworkErrorToStr` FailureType))))

(event `ShowMainMenu`
  (bind _mainmenuwidget (`self.MainMenuWidget`))
  ;[1 1 1] ShowMainMenu :: Affiche le menu principal
  (`/Engine/EditorBlueprintResources/StandardMacros.IsValid` _mainmenuwidget
    (:`Is Valid`
      _)
    (:`Is Not Valid`
      (bind _returnvalue (`|CreateWidget` "/Game/EqEngine/Blueprints/Menus/EQ_MainMenu.EQ_MainMenu_C" (`GameplayStatics.GetPlayerController` 0)))
      (set `self.MainMenuWidget` _returnvalue)))
  (`UserWidget.AddToViewport` _mainmenuwidget 0))

(event `self.HandleTravelError`
  (params (FailureType :type "ETravelFailure Enum" :default "NoLevel"))
  ;[1 1 1] Gère NetworkError & TravelError
  (`self.Error` (`self.TravelErrorToStr` FailureType)))

(event `HostGame`
  (params (MaxPlayers :type Integer) (`UseLAN?` :type Boolean) (ServerName :type Text))
  ;[1 1 1] HostGame :: Host une session Unreal
  (set `self.MaxPlayers` MaxPlayers)
  (set `self.ServerName` ServerName)
  (`self.ShowLoadingScreen`)
  (`CreateSessionCallbackProxy.CreateSession` null (`self.MaxPlayers`) `UseLAN?`
    (:`OnSuccess`
      (`GameplayStatics.OpenLevel` "FirstPersonExampleMap" true "listen"))
    (:`OnFailure`
      (`self.Error` "Error: Can't create UE4 Session, please try again."))))

(event `JoinGame`
  (params (TargetServer :type "BlueprintSessionResult Structure"))
  ;[1 1 1] JoinGame :: Rejoind une session Unreal
  (`self.ShowLoadingScreen`)
  (`JoinSessionCallbackProxy.JoinSession` (`GameplayStatics.GetPlayerController` 0) TargetServer
    (:`OnFailure`
      (`self.Error` "Error: Can't join server, please retry. "))))

(event `ShowLoadingScreen`
  (bind _loadingscreenwidget (`self.LoadingScreenWidget`))
  ;[1 1 1] ShowLoadingScreen :: Affiche l'écran de chargement
  (`/Engine/EditorBlueprintResources/StandardMacros.IsValid` _loadingscreenwidget
    (:`Is Valid`
      _)
    (:`Is Not Valid`
      (bind _returnvalue (`|CreateWidget` "/Game/EqEngine/Blueprints/Menus/EQ_LoadingScreen.EQ_LoadingScreen_C" (`GameplayStatics.GetPlayerController` 0)))
      (set `self.LoadingScreenWidget` _returnvalue)))
  (`UserWidget.AddToViewport` _loadingscreenwidget 0))

(event `DestroySession`
  (params (PlayerController :type "PlayerController Object Reference"))
  ;[1 1 1] DestroySession :: Détruit la session Unreal
  (`DestroySessionCallbackProxy.DestroySession` PlayerController))

(fn `NetworkErrorToStr`
  (params (Failure :type "ENetworkFailure Enum"))
  (returns (OutStr :type String))
  (return ""))

(fn `TravelErrorToStr`
  (params (Failure :type "ETravelFailure Enum"))
  (returns (OutStr :type String))
  (return ""))