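; Player controller that sets up the chat HUD and loads each player's social identity for the social system.
; On client load it links HUD widgets to SocialSystemComponent, then requests a server load with ID -1.
; The server copies name, guild and party data from GameState lists into PlayerState; the PlayerArray-index demo fallback sits behind an always-true check.
; Keys focus chat, prefill commands or track right mouse.
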(event `Client_LoadPlayer`
  (bind _hudreference (`self.HUDReference`))
  ;[0.2617 0.94 0.2491] Init Player
  ;[0.2617 0.94 0.2491] Setup HUD Reference
  (bind _returnvalue (`|CreateWidget` "/Game/AdvancedSocialSystem/UI/ChatHUDLayout.ChatHUDLayout_C" self))
  (bind _output_get (set `self.HUDReference` _returnvalue))
  (`UserWidget.AddToViewport` _output_get 0)
  (`WidgetBlueprintLibrary.SetInputMode_GameAndUIEx` self (`self.HUDReference`))
  (set `self.bShowMouseCursor` true)
  ;[0.2617 0.94 0.2491] Chat Component References
  (`/Game/AdvancedSocialSystem/Blueprints/Social/SocialSystemComponent.InitializeSocialSystemUI` (`self.SocialSystemComponent`) (`/Game/AdvancedSocialSystem/UI/ChatHUDLayout.ChatWindow` _hudreference) (`/Game/AdvancedSocialSystem/UI/ChatHUDLayout.PlayerFrame` _hudreference) (`/Game/AdvancedSocialSystem/UI/ChatHUDLayout.PartyFrames` _hudreference))
  (`self.Server_LoadPlayer` -1))

(event `Server_LoadPlayer`
  (params (PlayerID :type Integer))
  ;[0.845 0.1098 0.1098] DEMO [PLAY IN EDITOR ] Player ID -1 Automatically Loads Next Player In Player List On Join
  (`self.LoadPlayerInfo` PlayerID)
  ;[0.845 0.1098 0.1098] Demo: Client Welcome Message
  (`/Game/AdvancedSocialSystem/Blueprints/Social/SocialSystemComponent.OnPlayerLogin` (`self.SocialSystemComponent`)))

(event `/Game/EqEngine/Blueprints/Gameplay/BP_SocialInterface.UI_FocusChatInput`
  ;[0.1019 0.4359 0.885] Social UI Events
  (`Widget.SetUserFocus` (`/Game/AdvancedSocialSystem/UI/Blueprints/ChatWindow.InputText` (`/Game/AdvancedSocialSystem/UI/ChatHUDLayout.ChatWindow` (`self.HUDReference`))) self))

(event `/Game/EqEngine/Blueprints/Gameplay/BP_SocialInterface.UI_FocusChatCommand`
  (bind _inputtext (`/Game/AdvancedSocialSystem/UI/Blueprints/ChatWindow.InputText` (`/Game/AdvancedSocialSystem/UI/ChatHUDLayout.ChatWindow` (`self.HUDReference`))))
  ;[0.1019 0.4359 0.885] Social UI Events
  (`Widget.SetUserFocus` _inputtext self)
  (`EditableText.SetText` _inputtext "/"))

(event `Key|Enter`
  (params (Key :type "Key Structure" :default "AnyKey"))
  ;[0.1019 0.4359 0.885] Input: Chat
  (:`Pressed`
    (`self.UI_FocusChatInput`)))

(event `/Game/EqEngine/Blueprints/Gameplay/BP_SocialInterface.UI_FocusChatReply`
  (bind _inputtext (`/Game/AdvancedSocialSystem/UI/Blueprints/ChatWindow.InputText` (`/Game/AdvancedSocialSystem/UI/ChatHUDLayout.ChatWindow` (`self.HUDReference`))))
  ;[0.1019 0.4359 0.885] Social UI Events
  (`Widget.SetUserFocus` _inputtext self)
  (`EditableText.SetText` _inputtext "/r "))

(event `Key|Slash`
  (params (Key :type "Key Structure" :default "AnyKey"))
  ;[0.1019 0.4359 0.885] Input: Chat
  (:`Pressed`
    (`self.UI_FocusChatCommand`)))

(event `/Game/EqEngine/Blueprints/Gameplay/BP_SocialInterface.UI_RemoveChatFocus`
  ;[0.1019 0.4359 0.885] Social UI Events
  (`Widget.SetUserFocus` (`/Game/AdvancedSocialSystem/UI/ChatHUDLayout.ChatWindow` (`self.HUDReference`)) self))

(event `Key|R`
  (params (Key :type "Key Structure" :default "AnyKey"))
  ;[0.1019 0.4359 0.885] Input: Chat
  (:`Pressed`
    (`self.UI_FocusChatReply`)))

(event `Key|RightMouseButton`
  (params (Key :type "Key Structure" :default "AnyKey"))
  ;[0.1019 0.4359 0.885] Input: Mouse
  (:`Pressed`
    (set `self.IsRightMouseButtonDown` true))
  (:`Released`
    (set `self.IsRightMouseButtonDown` false)))

(fn `GetSocalComponent`
  (returns (`Social System Reference` :type "/Game/AdvancedSocialSystem/Blueprints/Social/SocialSystemComponent Object Reference"))
  (return (`self.SocialSystemComponent`)))

(fn `LoadPlayerInfo`
  (params (PlayerID :type Integer))
  ;[0.845 0.1098 0.1098] Load Player Info from Datatable
  (`/Engine/EditorBlueprintResources/ActorMacros.Switch Has Authority`
    (:`Authority`
      (if (>= 0 0)
        (set `self.LocalPlayerID` PlayerID)
        (else
          ;[0.845 0.1098 0.1098] DEMO [PLAY IN EDITOR ] Player ID -1 Automatically Loads Next Player In Player List On Join
          (for (_array_element _array_index) (`GameState.PlayerArray` (`GameplayStatics.GetGameState`))
            (if (== (`self.PlayerState`) _array_element)
              (set `self.LocalPlayerID` _array_index)
              (break)))))
      (bind _asbp_eqgame_state_base (cast `/Game/EqEngine/Blueprints/Gameplay/BP_EQGameStateBase` (`GameplayStatics.GetGameState`)))
      (bind _output_get (set `self.LocalSocialGameState` _asbp_eqgame_state_base))
      (bind _asbp_eqplayer_state (cast `/Game/EqEngine/Blueprints/Gameplay/BP_EQPlayerState` (`self.PlayerState`)))
      (bind (_id _name _guildid _partyid) (break `/Game/AdvancedSocialSystem/Blueprints/Social/SPlayer` (`KismetArrayLibrary.Array_Get` (`/Game/EqEngine/Blueprints/Gameplay/BP_EQGameStateBase.Players` _output_get) (`self.LocalPlayerID`))))
      (set `/Game/EqEngine/Blueprints/Gameplay/BP_EQPlayerState.SocialID` _id _asbp_eqplayer_state)
      (set `/Game/EqEngine/Blueprints/Gameplay/BP_EQPlayerState.SocialName` _name _asbp_eqplayer_state)
      (if (>= _guildid 0)
        (set `/Game/EqEngine/Blueprints/Gameplay/BP_EQPlayerState.GuildName` (`.Name_18_5DCF797749551705495DB986FC0E4195` (break `/Game/AdvancedSocialSystem/Blueprints/Social/SGuild` (`KismetArrayLibrary.Array_Get` (`/Game/EqEngine/Blueprints/Gameplay/BP_EQGameStateBase.Guilds` _output_get) _guildid))) _asbp_eqplayer_state)
        (else
          (set `/Game/EqEngine/Blueprints/Gameplay/BP_EQPlayerState.GuildName` "" _asbp_eqplayer_state)))
      (set `/Game/EqEngine/Blueprints/Gameplay/BP_EQPlayerState.GuildID` _guildid _asbp_eqplayer_state)
      (set `/Game/EqEngine/Blueprints/Gameplay/BP_EQPlayerState.PartyID` _partyid _asbp_eqplayer_state)
      (`/Game/EqEngine/Blueprints/Gameplay/BP_EQGameStateBase.UpdatePlayerStatus` (`self.LocalSocialGameState`) (`self.LocalPlayerID`) _asbp_eqplayer_state))))

(fn `UI_GetSocialState`
  (returns (SocialID :type Integer) (SocialName :type String) (PartyID :type Integer) (GuildID :type Integer) (GuildName :type String) (GeneralID :type Integer) (TradeID :type Integer))
  (bind _asbp_eqplayer_state (cast `/Game/EqEngine/Blueprints/Gameplay/BP_EQPlayerState` (`self.PlayerState`))
    (:`then`
      (return (`/Game/EqEngine/Blueprints/Gameplay/BP_EQPlayerState.SocialID` _asbp_eqplayer_state) (`/Game/EqEngine/Blueprints/Gameplay/BP_EQPlayerState.SocialName` _asbp_eqplayer_state) (`/Game/EqEngine/Blueprints/Gameplay/BP_EQPlayerState.PartyID` _asbp_eqplayer_state) (`/Game/EqEngine/Blueprints/Gameplay/BP_EQPlayerState.GuildID` _asbp_eqplayer_state) (`/Game/EqEngine/Blueprints/Gameplay/BP_EQPlayerState.GuildName` _asbp_eqplayer_state) (`/Game/EqEngine/Blueprints/Gameplay/BP_EQPlayerState.CurrentGeneralID` _asbp_eqplayer_state) (`/Game/EqEngine/Blueprints/Gameplay/BP_EQPlayerState.CurrentTradeID` _asbp_eqplayer_state)))
    (:`CastFailed`
      (return 0 "" 0 0 "" 0 0))))

(fn `UserConstructionScript`)