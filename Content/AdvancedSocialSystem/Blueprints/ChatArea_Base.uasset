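; Base chat area actor for the social system that moves characters in and out of zone-specific chat channels as they enter or leave it.
; Begin and end overlap events run authority-only functions that get the social component from the character's controller through a message call.
; That component sends the player an entered or left system message with the area name, then joins or leaves the General channel and, if enabled, the Trade channel.
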(event `self.ReceiveActorBeginOverlap`
  (params (OtherActor :type "Actor Object Reference"))
  ;[0.845 0.1098 0.1098] Server: On Player Enter Area
  (`self.PlayerEnterArea` OtherActor))

(event `self.ReceiveActorEndOverlap`
  (params (OtherActor :type "Actor Object Reference"))
  ;[0.845 0.1098 0.1098] Server: On Player Leave Area
  (`self.PlayerLeaveArea` OtherActor))

(fn `PlayerEnterArea`
  (params (Actor :type "Actor Object Reference"))
  (`/Engine/EditorBlueprintResources/ActorMacros.Switch Has Authority`
    (:`Authority`
      (bind _ascharacter (cast `Character` Actor))
      (bind _social_system_reference (message `/Game/EqEngine/Blueprints/Basic/BP_SocialInterface.GetSocalComponent` (`Pawn.GetController` _ascharacter)))
      (`/Game/AdvancedSocialSystem/Blueprints/Social/SocialSystemComponent.Client_ReceiveSystemMessage` _social_system_reference "NewEnumerator0" (`KismetStringLibrary.Concat_StrStr` "You have entered " (`KismetStringLibrary.Conv_NameToString` (`self.AreaName`))))
      (`/Game/AdvancedSocialSystem/Blueprints/Social/SocialSystemComponent.Server_JoinChannelID` _social_system_reference "NewEnumerator0" (`self.GeneralChannelID`))
      (if (`self.HasTradeChannel`)
        (`/Game/AdvancedSocialSystem/Blueprints/Social/SocialSystemComponent.Server_JoinChannelID` _social_system_reference "NewEnumerator1" (`self.TradeChannelID`))))))

(fn `PlayerLeaveArea`
  (params (Actor :type "Actor Object Reference"))
  (`/Engine/EditorBlueprintResources/ActorMacros.Switch Has Authority`
    (:`Authority`
      (bind _ascharacter (cast `Character` Actor))
      (bind _socialsystemreference (message `/Game/AdvancedSocialSystem/Blueprints/Social/SocialControllerInterface.GetSocialComponent` (`Pawn.GetController` _ascharacter)))
      (`/Game/AdvancedSocialSystem/Blueprints/Social/SocialSystemComponent.Client_ReceiveSystemMessage` _socialsystemreference "NewEnumerator0" (`KismetStringLibrary.Concat_StrStr` "You have left " (`KismetStringLibrary.Conv_NameToString` (`self.AreaName`))))
      (`/Game/AdvancedSocialSystem/Blueprints/Social/SocialSystemComponent.Server_LeaveChannelID` _socialsystemreference "NewEnumerator0" (`self.GeneralChannelID`))
      (if (`self.HasTradeChannel`)
        (`/Game/AdvancedSocialSystem/Blueprints/Social/SocialSystemComponent.Server_LeaveChannelID` _socialsystemreference "NewEnumerator1" (`self.TradeChannelID`))))))

(fn `UserConstructionScript`)